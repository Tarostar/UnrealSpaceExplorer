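; BP_SpaceExplorer is the player's space explorer, with a work-in-progress inventory, accumulated damage and debug keys.
; It sizes inventory and HUD on BeginPlay, toggles HUD panels, and turns hits into speed-based damage that only prints status.
; Cursor line traces are rechecked under authority for pickup, though that chain ends at a cast.
; Authority-gated events add items and swap slots using HUD hitbox state.
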(event `Key|#`
  ;[1 1 1] Set Invulnerable - Shield Test
  (:`Pressed`
    (set `self.bCanBeDamaged` false)
    (`KismetSystemLibrary.PrintString` "Invulnerable")))

(event `Key|RightBracket`
  ;[1 1 1] Set Invulnerable - Shield Test
  (:`Pressed`
    (set `self.bCanBeDamaged` true)
    (`KismetSystemLibrary.PrintString` "Can be damaged.")))

(event `InputAction|Inventory`
  ;[1 1 1] Interact Inventory HUD - TODO: flipflop must figure out which inventory is opened and set HUD inv size to this on A before toggeling open
  (:`Pressed`
    (bind _isa (`/Engine/EditorBlueprintResources/StandardMacros.FlipFlop`)
      (:`B`
        (message `/Game/HUD/BP_HUDInterface.Toggle Inventory` (`PlayerController.GetHUD` (`GameplayStatics.GetPlayerController` 0)) _isa)))))

(event `self.ReceiveAnyDamage`
  (params (Damage :type "Float (single-precision)") (DamageType :type "DamageType Object Reference") (InstigatedBy :type "Controller Object Reference") (DamageCauser :type "Actor Object Reference"))
  (bind _returnvalue (+ Damage (`self.CurrentDamage`)))
  (set `self.CurrentDamage` _returnvalue)
  ;[1 1 1] Reached Max Damage
  (if (>= _returnvalue (`self.MaxDamage`))
    (`KismetSystemLibrary.PrintString` "KaBoom!" true false)
    (else
      (`KismetSystemLibrary.PrintString` "All is well Captain." true false))))

(event `self.ReceiveBeginPlay`
  (bind _returnvalue (`GameplayStatics.GetPlayerController` 0))
  ;[0.6861 0.2576 1] Set Inventory Size
  (message `/Game/HUD/BP_HUDInterface.SetInventorySize` (`PlayerController.GetHUD` (`GameplayStatics.GetPlayerController` 0)) 50 5)
  (`KismetArrayLibrary.Array_Resize` (`self.Inventory`) (+ 50 5))
  ;[1 1 1] Enable Mouse Input
  (set `PlayerController.bShowMouseCursor` true _returnvalue)
  (set `PlayerController.bEnableClickEvents` true _returnvalue)
  (set `PlayerController.bEnableMouseOverEvents` true _returnvalue))

(event `self.ReceiveHit`
  (params (MyComp :type "PrimitiveComponent Object Reference") (Other :type "Actor Object Reference") (OtherComp :type "PrimitiveComponent Object Reference") (bSelfMoved :type Boolean) (HitLocation :type "Object.Vector Structure") (HitNormal :type "Object.Vector Structure") (NormalImpulse :type "Object.Vector Structure") (Hit :type "EngineTypes.HitResult Structure (by ref)"))
  ;[1 1 1] Something hit us.
  (`GameplayStatics.ApplyPointDamage` self (`self.CurrentForwardSpeed`) (`self.GetActorForwardVector`) (`self.HitResult`)))

(event `self.ReceiveActorBeginOverlap`
  (params (OtherActor :type "Actor Object Reference"))
  ;[1 1 1] Server-Client Item Pickup
  ;;[0 0 0] Temporary Collision test code
  (if (== OtherActor "/Game/Blueprints/BP_BaseItemPlaceholder_Laser.BP_BaseItemPlaceholder_Laser")
    (`KismetSystemLibrary.PrintString` "HelloCollision")))

(event `Key|M`
  (bind _returnvalue (`GameplayStatics.GetPlayerController` 0))
  ;[1 1 1] Toggle Main Menu
  (:`Pressed`
    (message `/Game/HUD/BP_HUDInterface.Toggle menu` (`PlayerController.GetHUD` _returnvalue) true)
    (set `PlayerController.bShowMouseCursor` true _returnvalue)
    (set `PlayerController.bEnableClickEvents` true _returnvalue)
    (`self.EnableInput` _returnvalue)
    (`GameplayStatics.SetGamePaused` true)))

(event `InputAction|InteractWithItem`
  (bind (_worldlocation _worlddirection) (`PlayerController.DeprojectMousePositionToWorld` (`GameplayStatics.GetPlayerController` 0)))
  ;[1 1 1] Server-Client Item Pickup
  ;;[0.866 0.4615 1] Local call for raycast send to server
  (:`Pressed`
    (bind (_hit _objecthitactor) (`self.CheckTraceHit` _worldlocation _worlddirection))
    (if _hit
      (`/Engine/EditorBlueprintResources/StandardMacros.IsValid` _objecthitactor
        (:`Is Valid`
          (`self.PickupItem` _worldlocation _worlddirection))))))

(event `PickupItem`
  (params (WorldLoc :type "Object.Vector Structure") (WorldDir :type "Object.Vector Structure"))
  ;[1 1 1] Server-Client Item Pickup
  ;;[0.7789 0.5196 1] Server check for trace hit + destroy actor
  (`/Engine/EditorBlueprintResources/ActorMacros.Switch Has Authority`
    (:`Authority`
      (`self.ServerAttemptHitTrace` WorldLoc WorldDir))))

(event `UpdateInventoryItemsViaHUD`
  ;[1 1 1] Switching / adding / removing items from invetory
  (`/Engine/EditorBlueprintResources/ActorMacros.Switch Has Authority`
    (:`Authority`
      (`self.DetermineHitBox`))))

(event `DetermineHitBox`
  ;[1 1 1] Switching / adding / removing items from invetory
  (bind (_buttonpressed _buttonhighlighted) (`self.GetHitBoxInfoFromHUD`))
  (`self.UpdateHitBoxInfo` _buttonpressed _buttonhighlighted))

(event `SendDestroyToItemFromLocal`
  (params (ItemIn :type "Actor Object Reference"))
  ;[1 1 1] Server-Client Item Pickup
  ;;[0.7843 0.1632 1] Send item from character
  (bind _asbp_usableobject_c (cast `/Game/Items/BP_UsableObject` ItemIn)))

(event `UpdateHitBoxInfo`
  (params (ButtonPressed :type Integer) (ButtonHighlighted :type Integer))
  ;[1 1 1] Switching / adding / removing items from invetory
  (`self.SwitchItemInInventory` ButtonPressed ButtonHighlighted))

(event `AddObjectToInventory`
  (params (ItemClass :type "UsableObject Object Reference"))
  ;[1 1 1] Server-Client Item Pickup
  ;;[0.5982 0.4273 1] Event called to place items in inventory
  ;[1 0.055 0.055] DEBUG
  (`KismetSystemLibrary.PrintString` (`KismetStringLibrary.Concat_StrStr` "PlaceItemInInventory on" (`KismetMathLibrary.SelectString` "Server" "Client" (`KismetSystemLibrary.IsServer`))) false)
  (`/Engine/EditorBlueprintResources/ActorMacros.Switch Has Authority`
    (:`Authority`
      (bind _returnvalue (`self.AddItem` ItemClass))
      (if _returnvalue
        (`UsableObject.Collect` ItemClass self)
        (`KismetSystemLibrary.PrintString` "Item Added")
        (else
          (`KismetSystemLibrary.PrintString` "NO FREE SPACE!"))))))

(fn `CheckTraceHit`
  (params (WorldLoc :type "Object.Vector Structure") (WorldDir :type "Object.Vector Structure"))
  (returns (Hit :type Boolean) (ObjectHitActor :type "Actor Object Reference"))
  (bind (_outhit _returnvalue) (`KismetSystemLibrary.LineTraceSingle` :`Start` WorldLoc :`End` (+ WorldLoc (* WorldDir 10000.0)) :`TraceChannel` "TraceTypeQuery1" :`bTraceComplex` true :`DrawDebugType` "Persistent"))
  (return _returnvalue (`.HitActor` (`GameplayStatics.BreakHitResult` _outhit))))

(fn `GetHitBoxInfoFromHUD`
  (returns (ButtonPressed :type Integer) (ButtonHighlighted :type Integer))
  (bind _asbp_customhud_c (cast `/Game/HUD/BP_CustomHUD` (`PlayerController.GetHUD` (`GameplayStatics.GetPlayerController` 0))))
  (return (`/Game/HUD/BP_CustomHUD.HitboxToInt` _asbp_customhud_c) (`/Game/HUD/BP_CustomHUD.HitboxHighlighted` _asbp_customhud_c)))

(fn `ServerAttemptHitTrace`
  (params (WorldLoc :type "Object.Vector Structure") (WorldDir :type "Object.Vector Structure"))
  (`/Engine/EditorBlueprintResources/ActorMacros.Switch Has Authority`
    (:`Authority`
      (bind (_hit _objecthitactor) (`self.CheckTraceHit` WorldLoc WorldDir))
      ;[0.7452 0.2602 1] Trace Hit?
      (if _hit
        ;[0.6704 0.2069 1] Valid Object?
        (`/Engine/EditorBlueprintResources/StandardMacros.IsValid` _objecthitactor
          (:`Is Valid`
            ;[0.3543 0.03491 1] Is Placeholder Item Child?
            (if (`KismetMathLibrary.ClassIsChildOf` (`GameplayStatics.GetObjectClass` _objecthitactor) "/Script/SpaceExplorer.UsableObject")
              (`self.SendDestroyToItemFromLocal` _objecthitactor))))))))

(fn `SwitchItemInInventory`
  (params (ButtonPressed :type Integer) (ButtonHighlighted :type Integer))
  (bind _inventory (`self.Inventory`))
  (if (not (== ButtonPressed ButtonHighlighted))
    (bind _asbp_customhud_c (cast `/Game/HUD/BP_CustomHUD` (`PlayerController.GetHUD` (`GameplayStatics.GetPlayerController` 0))))
    (`KismetArrayLibrary.Array_Set` _inventory ButtonPressed (`KismetArrayLibrary.Array_Get` _inventory ButtonHighlighted))
    (`KismetArrayLibrary.Array_Set` _inventory ButtonHighlighted (`/Game/HUD/BP_CustomHUD.ItemBeingMoved` _asbp_customhud_c))))

(fn `UserConstructionScript`)